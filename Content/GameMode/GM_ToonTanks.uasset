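; GM_ToonTanks is the Toon Tanks game mode Blueprint that shows the match's start and end screens.
; StartGame adds a WBP_Start widget for player 0 to the viewport, then runs a three-second Delay with nothing after it.
; EndGame adds a WBP_End widget, setting its EndText to a win or retry message from the WonGame flag.
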(event `self.StartGame`
  (bind _returnvalue (`|CreateWidget` "/Game/Blueprints/UI/WBP_Start.WBP_Start_C" (`GameplayStatics.GetPlayerController` 0)))
  (`UserWidget.AddToViewport` _returnvalue 0)
  (`KismetSystemLibrary.Delay` 3.0))

(event `self.EndGame`
  (params (bWonGame :type Boolean))
  (bind _returnvalue (`|CreateWidget` "/Game/Blueprints/UI/WBP_End.WBP_End_C" (`GameplayStatics.GetPlayerController` 0)))
  (`TextBlock.SetText` (`/Game/Blueprints/UI/WBP_End.EndText` _returnvalue) (select `bool` bWonGame :`false` "Try Again?" :`true` "You Won!" :!type "Text"))
  (`UserWidget.AddToViewport` _returnvalue 0))

(fn `UserConstructionScript`)